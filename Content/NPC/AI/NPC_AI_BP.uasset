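; AI controller for guard NPCs that runs the GuardBehavior tree on the PatrolData blackboard.
; AI perception writes any sensed actor not tagged "Enemy" to EnemyKey and clears the key when such an actor is lost.
; Each tick, it sets the controlled PatrollingGuardV2's aiming and shooting flags according to whether the controller has a valid focus actor.
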(event `self.AIPerception.OnTargetPerceptionUpdated`
  (params (Actor :type "Actor Object Reference") (Stimulus :type "AIStimulus Structure"))
  (bind _enemykey (`self.EnemyKey`))
  (bind _blackboard_component (`self.Blackboard Component`))
  (if (`self.ActorHasTag` Actor "Enemy")
    _
    (elif (`.bSuccessfullySensed` (break `AIStimulus` Stimulus))
      (`BlackboardComponent.SetValueAsObject` _blackboard_component _enemykey Actor)
      (else
        (`BlackboardComponent.ClearValue` _blackboard_component _enemykey)))))

(event `self.ReceiveBeginPlay`
  (bind _blackboardcomponent (`self.UseBlackboard` "/Game/NPC/AI/PatrolData.PatrolData"))
  (`self.RunBehaviorTree` "/Game/NPC/AI/GuardBehavior.GuardBehavior")
  (set `self.Blackboard Component` _blackboardcomponent))

(event `self.ReceiveTick`
  (params (DeltaSeconds :type "Float (single-precision)"))
  (bind _returnvalue (`KismetSystemLibrary.IsValid` (`self.GetFocusActor`)))
  (bind _aspatrolling_guard_v2 (cast `/Game/NPC/Character/PatrollingGuardV2` (`self.K2_GetPawn`)))
  (set `/Game/NPC/Character/PatrollingGuardV2.AimingDown` _returnvalue _aspatrolling_guard_v2)
  (set `/Game/NPC/Character/PatrollingGuardV2.ShootingDown` _returnvalue _aspatrolling_guard_v2))

(fn `UserConstructionScript`)